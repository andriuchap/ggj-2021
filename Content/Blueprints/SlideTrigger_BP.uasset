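; SlideTrigger_BP is a trigger volume that temporarily changes how a Character_BP moves while inside it, apparently for a slide area.
; On begin overlap it caches the character and its original max acceleration and walk speed, then applies the trigger's configured values.
; On end overlap it restores the cached values if the leaving actor is the cached character.
; It tracks only one character at a time.
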(event OnComponentBeginOverlap(CollisionComponent)
  (params (OverlappedComponent :type Primitive%20Component%20Object%20Reference) (OtherActor :type Actor%20Object%20Reference) (OtherComp :type Primitive%20Component%20Object%20Reference) (OtherBodyIndex :type Integer) (bFromSweep :type Boolean) (SweepResult :type Hit%20Result%20Structure%20%28by%20ref%29))
  (bind _ascharacter_bp (Utilities|Casting|CastToCharacter_BP OtherActor))
  (bind _output_get (Variables|Default|SetCurrentChar _ascharacter_bp))
  (Variables|Default|SetOriginalAcceleration (Variables|/Script/Engine.CharacterMovementComponent|GetMaxAcceleration (Variables|/Script/Engine.Character|GetCharacterMovement _output_get)))
  (Variables|Default|SetOriginalMaxSpeed (Variables|/Script/Engine.CharacterMovementComponent|GetMaxWalkSpeed (Variables|/Script/Engine.Character|GetCharacterMovement _output_get)))
  (Variables|/Script/Engine.CharacterMovementComponent|SetMaxAcceleration (Variables|/Script/Engine.Character|GetCharacterMovement _output_get) (Variables|Default|GetSetMaxAcceleration))
  (Variables|/Script/Engine.CharacterMovementComponent|SetMaxWalkSpeed (Variables|/Script/Engine.Character|GetCharacterMovement _output_get) (Variables|Default|GetSetMaxSpeed)))

(event OnComponentEndOverlap(CollisionComponent)
  (params (OverlappedComponent :type Primitive%20Component%20Object%20Reference) (OtherActor :type Actor%20Object%20Reference) (OtherComp :type Primitive%20Component%20Object%20Reference) (OtherBodyIndex :type Integer))
  (bind _currentchar (Variables|Default|GetCurrentChar))
  (bind _charactermovement (Variables|/Script/Engine.Character|GetCharacterMovement _currentchar))
  (if (== OtherActor _currentchar)
    (Variables|/Script/Engine.CharacterMovementComponent|SetMaxAcceleration _charactermovement (Variables|Default|GetOriginalAcceleration))
    (Variables|/Script/Engine.CharacterMovementComponent|SetMaxWalkSpeed _charactermovement (Variables|Default|GetOriginalMaxSpeed))))

(event EventBeginPlay)

(event Collision|EventActorBeginOverlap
  (params (OtherActor :type Actor%20Object%20Reference)))

(event EventTick
  (params (DeltaSeconds :type Float%20%28single-precision%29)))

(fn ConstructionScript)