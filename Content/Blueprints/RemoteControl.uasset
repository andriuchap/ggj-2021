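; RemoteControl is a two-button controller that drives a referenced Car actor back and forth along the world Y axis.
; Overlapping LeftBtn or RightBtn sets that direction's drive flag and plays a shared press cue, and ending the overlap clears the flag.
; Each Tick, active flags apply swept, frame-rate-independent location offsets scaled by DriveSpeed, with left as +Y and right as -Y.
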(event OnComponentBeginOverlap(LeftBtn)
  (params (OverlappedComponent :type Primitive%20Component%20Object%20Reference) (OtherActor :type Actor%20Object%20Reference) (OtherComp :type Primitive%20Component%20Object%20Reference) (OtherBodyIndex :type Integer) (bFromSweep :type Boolean) (SweepResult :type Hit%20Result%20Structure%20%28by%20ref%29))
  (Variables|Default|SetDriveLeft true)
  (Audio|Components|Audio|Play (Variables|Default|GetButtonPress_Cue) 0.0))

(event OnComponentEndOverlap(LeftBtn)
  (params (OverlappedComponent :type Primitive%20Component%20Object%20Reference) (OtherActor :type Actor%20Object%20Reference) (OtherComp :type Primitive%20Component%20Object%20Reference) (OtherBodyIndex :type Integer))
  (Variables|Default|SetDriveLeft false))

(event OnComponentBeginOverlap(RightBtn)
  (params (OverlappedComponent :type Primitive%20Component%20Object%20Reference) (OtherActor :type Actor%20Object%20Reference) (OtherComp :type Primitive%20Component%20Object%20Reference) (OtherBodyIndex :type Integer) (bFromSweep :type Boolean) (SweepResult :type Hit%20Result%20Structure%20%28by%20ref%29))
  (Variables|Default|SetDriveRight true)
  (Audio|Components|Audio|Play (Variables|Default|GetButtonPress_Cue) 0.0))

(event OnComponentEndOverlap(RightBtn)
  (params (OverlappedComponent :type Primitive%20Component%20Object%20Reference) (OtherActor :type Actor%20Object%20Reference) (OtherComp :type Primitive%20Component%20Object%20Reference) (OtherBodyIndex :type Integer))
  (Variables|Default|SetDriveRight false))

(event EventTick
  (params (DeltaSeconds :type Float%20%28single-precision%29))
  (bind _car (Variables|Default|GetCar))
  (bind _drivespeed (Variables|Default|GetDriveSpeed))
  (bind _returnvalue (Transformation|GetActorLocation _car))
  (bind _returnvalue_2 (* DeltaSeconds _drivespeed))
  (Utilities|FlowControl|Sequence
    (:then_0
      (if (Variables|Default|GetDriveLeft)
        (Transformation|SetActorLocation _car (+ _returnvalue (Math|Vector|MakeVector 0.0 _returnvalue_2 0.0)) true false)))
    (:then_1
      (if (Variables|Default|GetDriveRight)
        (Transformation|SetActorLocation _car (+ _returnvalue (Math|Vector|MakeVector 0.0 (* _returnvalue_2 -1.0) 0.0)) true false)))))

(fn ConstructionScript)